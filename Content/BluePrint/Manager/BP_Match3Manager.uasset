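; Match-3 manager that turns board events into HUD animations and effects on the player ship and two AI ships.
; On board init it caches the HUD and tag-identified ships.
; Clear and fall handlers play visuals, then call AdvanceGameState after fixed delays to pace the board.
; Skill casts route East Wind to the caster and other handled skills to both rival ships; number keys are hardwired skill tests.
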(event EventOnPlayerSpeedUpTriggered
  (params (TriggerCount :type Integer) (SpeedBoostAmount :type Float%20%28single-precision%29))
  (Utilities|FlowControl|Delay 0.4)
  (bind _playership (Variables|ActorInMap|GetPlayerShip)
    (:then
      (Default|EventGetSpeedUP _playership TriggerCount SpeedBoostAmount)
      (Default|FCreatEffectUI (Variables|Default|GetHUD) (.ScreenPosition (Class|GameplayStatics|ProjectWorldtoScreen (Game|GetPlayerController 0) (Transformation|GetWorldLocation (Variables|/Game/LxsTestData/BP_Basic/BP_Ship.BP_Ship_C|GetUIPos_0 (Variables|ActorInMap|GetPlayerShip))) true))))
    (:else)))

(event EventOnMoraleChanged
  (params (NewMorale :type Integer) (InMaxMorale :type Integer) (AddedAmount :type Integer))
  (Development|PrintString (Utilities|String|Append "士气变化" (Utilities|String|ToString(Integer) NewMorale)))
  (bind _hud (Variables|Default|GetHUD)
    (:then
      (Default|EventUPDataMorale (Variables|/Game/UMG/WBP_HUD.WBP_HUD_C|GetWBP_BoardAndSkill _hud) NewMorale InMaxMorale))
    (:else)))

(event EventOnSkillCasted
  (params (SkillType :type ESkillType%20Enum :default "EastWind") (Config :type Skill%20Config%20Structure%20%28by%20ref%29))
  ;[1 1 1] 玩家释放技能
  (CallFunction|FPlayerApplyEffect SkillType Config)
  (Default|EventCallSikllBoBao (Variables|/Game/UMG/WBP_HUD.WBP_HUD_C|GetWBP_特效层 (Variables|Default|GetHUD)) SkillType 1))

(event EventOnAISkillCasted
  (params (CasterAI :type EAIBoatIndex%20Enum :default "AI1") (SkillType :type ESkillType%20Enum :default "EastWind") (TargetType :type ESkillTargetType%20Enum :default "Self") (TargetAI :type EAIBoatIndex%20Enum :default "AI1") (bTargetIsPlayer :type Boolean) (Config :type Skill%20Config%20Structure%20%28by%20ref%29))
  (bind _hud (Variables|Default|GetHUD))
  (bind _wbp_特效层 (Variables|/Game/UMG/WBP_HUD.WBP_HUD_C|GetWBP_特效层 _hud))
  ;[1 1 1] AI释放技能
  (CallFunction|FAISkill CasterAI SkillType TargetType Config)
  (if (not (Variables|Default|GetEndSkillApply))
    (switch Utilities|FlowControl|Switch|SwitchonEAIBoatIndex CasterAI
      (:AI1
        (Default|EventCallSikllBoBao _wbp_特效层 SkillType 1))
      (:AI2
        (Default|EventCallSikllBoBao _wbp_特效层 SkillType 2)))))

(event EventOnSpecialAreasUpdated
  (Default|FInitial (Variables|/Game/UMG/WBP_HUD.WBP_HUD_C|GetWBP_PlotsOverlay (Variables|Default|GetHUD)))
  (Development|PrintString (Utilities|String|ToString(Integer) (Utilities|Array|Length (Variables|Default|GetSpecialAreaGrid)))))

(event EventOnMatchesCleared
  (params (ClearedIndices :type Array%20of%20Integers) (TriggeredEffects :type Array%20of%20Special%20Effect%20Data%20Structures))
  (bind _hud (Variables|Default|GetHUD)
    (:then
      (Default|FHandleClearAnimi (Variables|/Game/UMG/WBP_HUD.WBP_HUD_C|GetWBP_PlotsOverlay _hud) ClearedIndices)
      (Default|FHandleEffect _hud TriggeredEffects (.ScreenPosition (Class|GameplayStatics|ProjectWorldtoScreen (Game|GetPlayerController 0) (Transformation|GetActorLocation (Variables|ActorInMap|GetPlayerShip)) true)))
      (Audio|PlaySound2D "/Game/Assets/WAV/正常消除01.正常消除01" 1.0 1.0 0.0 0 0)
      (Utilities|FlowControl|Delay 0.4)
      (Class|Datamanagement|AdvanceGameState))
    (:else)))

(event EventBeginPlay)

(event EventOnBoardInitialized
  (Utilities|FlowControl|Delay 0.1)
  (Utilities|FlowControl|Sequence
    (:then_0
      (bind _foundwidgets (Widget|GetAllWidgetsOfClass "/Game/UMG/WBP_HUD.WBP_HUD_C" false))
      (Variables|Default|SetHUD (Utilities|Array|Get(acopy) _foundwidgets)))
    (:then_1
      (bind _outactors (Actor|GetAllActorsOfClass "/Game/LxsTestData/BP_Basic/BP_Ship.BP_Ship_C"))
      (for _array_element _outactors
        (Utilities|FlowControl|Sequence
          (:then_0
            (if (Actor|ActorHasTag _array_element "Player")
              (Variables|ActorInMap|SetPlayerShip _array_element)))
          (:then_1
            (if (Actor|ActorHasTag _array_element "AI01")
              (Variables|ActorinMap|SetAIShip01 _array_element)))
          (:then_2
            (if (Actor|ActorHasTag _array_element "AI02")
              (Variables|ActorinMap|SetAIShip02 _array_element))))))))

(event EventOnBoardReshuffle
  (Development|PrintString "死锁" true true "(R=1.000000,G=0.000000,B=0.228147,A=1.000000)" 1e+01))

(event EventOnFallAnimTriggered
  (params (FallMoves :type Array%20of%20Fall%20Move%20Structures))
  (bind _hud (Variables|Default|GetHUD)
    (:then
      (Default|FHandleFallData (Variables|/Game/UMG/WBP_HUD.WBP_HUD_C|GetWBP_PlotsOverlay _hud) FallMoves)
      (Utilities|FlowControl|Delay 0.3)
      (Class|Datamanagement|AdvanceGameState))
    (:else)))

(event EventOnSwapAnimTriggered
  (params (IndexA :type Integer) (IndexB :type Integer) (bIsSuccessful :type Boolean))
  (if bIsSuccessful
    (bind _hud (Variables|Default|GetHUD)
      (:then
        (Default|FSworp (Variables|/Game/UMG/WBP_HUD.WBP_HUD_C|GetWBP_PlotsOverlay _hud) IndexA IndexB false))
      (:else))
    (else
      (Development|PrintString "失败")
      (bind _hud_2 (Variables|Default|GetHUD)
        (:then
          (Default|FSworp (Variables|/Game/UMG/WBP_HUD.WBP_HUD_C|GetWBP_PlotsOverlay _hud_2) IndexA IndexB false)
          (Utilities|FlowControl|Delay 0.2)
          (Default|FSworp (Variables|/Game/UMG/WBP_HUD.WBP_HUD_C|GetWBP_PlotsOverlay _hud_2) IndexB IndexA false))
        (:else)))))

(event EventOnSkillPointChanged
  (params (NewSkillPoints :type Integer) (InMaxSkillPoints :type Integer))
  (Development|PrintString "技能点变化" true true "(R=0.000000,G=1.000000,B=0.207158,A=1.000000)" 1e+01)
  (bind _hud (Variables|Default|GetHUD)
    (:then
      (Default|EventUPdataSkillPoint (Variables|/Game/UMG/WBP_HUD.WBP_HUD_C|GetWBP_BoardAndSkill _hud) NewSkillPoints))
    (:else)))

(event EventOnPlayerSlowDownEnemyTriggered
  (params (TriggerCount :type Integer) (SlowDownAmount :type Float%20%28single-precision%29))
  (Default|EventGetSpeedDown (Variables|ActorinMap|GetAIShip01) TriggerCount SlowDownAmount))

(event Input|KeyboardEvents|5
  (params (Key :type Key%20Structure :default "None"))
  (:Pressed
    (Default|EventApplySkill (Variables|ActorInMap|GetPlayerShip) "EmptyCity" (Utilities|Struct|MakeSkillConfig 5e+01 1e+03) false)))

(event Input|KeyboardEvents|2
  (params (Key :type Key%20Structure :default "None"))
  (:Pressed
    (Default|EventApplySkill (Variables|ActorInMap|GetPlayerShip) "FloodSeven" (Utilities|Struct|MakeSkillConfig 5.0 5.0) false)))

(event Input|KeyboardEvents|1
  (params (Key :type Key%20Structure :default "None"))
  (:Pressed
    (Default|EventApplySkill (Variables|ActorInMap|GetPlayerShip) "IronChain" (Utilities|Struct|MakeSkillConfig 5.0 15.0) false)))

(event Input|KeyboardEvents|3
  (params (Key :type Key%20Structure :default "None"))
  (:Pressed
    (Default|EventApplySkill (Variables|ActorInMap|GetPlayerShip) "EastWind" (Utilities|Struct|MakeSkillConfig 5.0 1e+03) false)))

(event Input|KeyboardEvents|6
  (params (Key :type Key%20Structure :default "None"))
  (:Pressed
    (Default|EventCallSikllBoBao (Variables|/Game/UMG/WBP_HUD.WBP_HUD_C|GetWBP_特效层 (Variables|Default|GetHUD)) "EastWind")))

(event Input|KeyboardEvents|4
  (params (Key :type Key%20Structure :default "None"))
  (:Pressed
    (Default|EventApplySkill (Variables|ActorInMap|GetPlayerShip) "HeavyFog" (Utilities|Struct|MakeSkillConfig 5.0 1e+03) false)))

(fn ConstructionScript)

(fn FPlayerApplyEffect
  (params (InputSkillType :type ESkillType%20Enum :default "EastWind") (SkillConfig :type Skill%20Config%20Structure))
  (Development|PrintString (Utilities|String|Append "触发技能" (Utilities|String|EnumtoString InputSkillType)) true true "(R=1.000000,G=0.000000,B=0.179855,A=1.000000)" 1e+01 "触发技能调试")
  (switch Utilities|FlowControl|Switch|SwitchonESkillType InputSkillType
    (:EastWind
      (Default|EventApplySkill (Variables|ActorInMap|GetPlayerShip) "EastWind" SkillConfig false))
    (:FloodSeven
      (Default|EventApplySkill (Variables|ActorinMap|GetAIShip01) InputSkillType SkillConfig false :!label _label))
    (:HeavyFog
      (goto _label))
    (:IronChain
      (goto _label))
    (:EmptyCity)))

(fn FAISkill
  (params (CastAI :type EAIBoatIndex%20Enum :default "AI1") (SkillType :type ESkillType%20Enum :default "EastWind") (TargetType :type ESkillTargetType%20Enum :default "Self") (SkillConfig :type Skill%20Config%20Structure%20%28by%20ref%29))
  (switch Utilities|FlowControl|Switch|SwitchonESkillType SkillType
    (:EastWind
      (switch Utilities|FlowControl|Switch|SwitchonEAIBoatIndex CastAI
        (:AI1
          (Default|EventApplySkill (Variables|ActorinMap|GetAIShip01) SkillType SkillConfig false))
        (:AI2
          (Default|EventApplySkill (Variables|ActorinMap|GetAIShip02) SkillType SkillConfig false))))
    (:FloodSeven
      (switch Utilities|FlowControl|Switch|SwitchonEAIBoatIndex CastAI :!label _label
        (:AI1
          (Default|EventApplySkill (Variables|ActorinMap|GetAIShip02) SkillType SkillConfig false)
          (Default|EventApplySkill (Variables|ActorInMap|GetPlayerShip) SkillType SkillConfig false))
        (:AI2
          (Default|EventApplySkill (Variables|ActorinMap|GetAIShip01) SkillType SkillConfig false)
          (Default|EventApplySkill (Variables|ActorInMap|GetPlayerShip) SkillType SkillConfig false))))
    (:HeavyFog
      (goto _label))
    (:IronChain
      (goto _label))))