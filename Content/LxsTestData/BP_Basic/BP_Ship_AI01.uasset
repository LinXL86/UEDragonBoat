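; AI opponent ship for a race that repeatedly chooses to idle, speed itself up or slow every other ship.
; On BeginPlay it gathers the other BP_Ship actors as targets and finds the one tagged Player.
; After race start, a delayed turn loop acts until RaceEnd, using a weighted random pick from FGetNextAction.
; The weights rubber-band on X distance to the player: slowing when ahead, boosting when behind, offset by difficulty.
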(event Custom|Event_NextTurn
  (if (not (Variables|Default|GetRaceEnd))
    (Utilities|FlowControl|Delay 1.0)
    (if (not (Variables|Default|GetRaceEnd))
      (switch int (CallFunction|FGetNextAction)
        (:0
          (Development|PrintString (Utilities|String|Append (Utilities|GetDisplayName self) "什么都没做")))
        (:1
          (CallFunction|EventGetSpeedUP (Math|Random|RandomIntegerinRange 1 3) (Variables|Default|GetAISpeedUPAmount))
          (Development|PrintString (Utilities|String|Append (Utilities|GetDisplayName self) "执行加速")))
        (:2
          (for _array_element (Variables|Default|GetAttackTarget)
            (Default|EventGetSpeedDown _array_element (Math|Random|RandomIntegerinRange 1 3) (Variables|Default|GetAISpeedDownAmount)))))
      (Utilities|FlowControl|Delay (Math|Random|RandomFloatinRange (Variables|Default|GetMinDelayTime) (Variables|Default|GetMaxDelayTime)))
      (if (not (Variables|Default|GetRaceEnd))
        (CallFunction|EventNextTurn)))))

(event EventBeginPlay
  (|CallParentFunction)
  (bind _outactors (Actor|GetAllActorsOfClass "/Game/LxsTestData/BP_Basic/BP_Ship.BP_Ship_C"))
  (for _array_element _outactors
    (Utilities|FlowControl|Sequence
      (:then_0
        (if (not (== _array_element self))
          (Utilities|Array|Add (Variables|Default|GetAttackTarget) _array_element)))
      (:then_1
        (if (Actor|ActorHasTag _array_element "Player")
          (Variables|Default|SetPlayerShip _array_element))))))

(event Collision|EventActorBeginOverlap
  (params (OtherActor :type Actor%20Object%20Reference))
  (|CallParentFunction OtherActor) ; 此节点被禁用，将不会被调用。\n从引脚连出引线来编译功能。
)

(event EventTick
  (params (DeltaSeconds :type Float%20%28single-precision%29))
  (|CallParentFunction DeltaSeconds) ; 此节点被禁用，将不会被调用。\n从引脚连出引线来编译功能。
)

(event EventEventStartRace
  (|CallParentFunction)
  (Utilities|FlowControl|Delay 1.0)
  (if (not (Variables|Default|GetRaceEnd))
    (switch int (CallFunction|FGetNextAction)
      (:0
        (Development|PrintString (Utilities|String|Append (Utilities|GetDisplayName self) "什么都没做")))
      (:1
        (CallFunction|EventGetSpeedUP (Math|Random|RandomIntegerinRange 1 3) (Variables|Default|GetAISpeedUPAmount))
        (Development|PrintString (Utilities|String|Append (Utilities|GetDisplayName self) "执行加速")))
      (:2
        (for _array_element (Variables|Default|GetAttackTarget)
          (Default|EventGetSpeedDown _array_element (Math|Random|RandomIntegerinRange 1 3) (Variables|Default|GetAISpeedDownAmount)))))
    (Utilities|FlowControl|Delay (Math|Random|RandomFloatinRange (Variables|Default|GetMinDelayTime) (Variables|Default|GetMaxDelayTime)))
    (if (not (Variables|Default|GetRaceEnd))
      (CallFunction|EventNextTurn))))

(fn ConstructionScript
  (|CallParentFunction))

(fn FGetNextAction
  (LocalVariables|SetActionWeight (Variables|Default|GetBasicWeightSet))
  (LocalVariables|SetNowDis (- (.x (Transformation|GetActorLocation)) (.x (Transformation|GetActorLocation (Variables|Default|GetPlayerShip)))))
  (Utilities|FlowControl|Sequence
    (:then_0
      (if (and (< (LocalVariables|GetNowDis) 2e+03) (>= (LocalVariables|GetNowDis) 1e+03))
        (Utilities|Array|SetArrayElem (LocalVariables|GetActionWeight) 2 (+ (Variables|Default|GetDiffcultyAdd) 5))))
    (:then_1
      (if (and (< (LocalVariables|GetNowDis) 1e+03) (>= (LocalVariables|GetNowDis) 0.0))
        (Utilities|Array|SetArrayElem (LocalVariables|GetActionWeight) 2 (+ (Variables|Default|GetDiffcultyAdd) 10))))
    (:then_2
      (if (and (< (LocalVariables|GetNowDis) 0.0) (>= (LocalVariables|GetNowDis) -1e+03))
        (Utilities|Array|SetArrayElem (LocalVariables|GetActionWeight) 1 (+ (Variables|Default|GetDiffcultyAdd) 20))))
    (:then_3
      (if (and (< (LocalVariables|GetNowDis) -1e+03) (>= (LocalVariables|GetNowDis) -2e+03))
        (Utilities|Array|SetArrayElem (LocalVariables|GetActionWeight) 1 (+ (Variables|Default|GetDiffcultyAdd) 40))))
    (:then_4
      (for _array_element (LocalVariables|GetActionWeight)
        (LocalVariables|SetMaxCount (+ (LocalVariables|GetMaxCount) _array_element)))
      (LocalVariables|SetGetCheckNum (Math|Random|RandomIntegerinRange 0 (LocalVariables|GetMaxCount)))
      (bind (_array_element_2 _array_index) (Utilities|Array|ForEachLoopwithBreak (LocalVariables|GetActionWeight) :!label _label)
        (:LoopBody
          (if (>= (LocalVariables|GetGetCheckNum) _array_element_2)
            (LocalVariables|SetGetCheckNum (- (LocalVariables|GetGetCheckNum) _array_element_2))
            (else
              (LocalVariables|SetGetIndex _array_index)
              (goto _label Break))))
        (:Completed
          (return (LocalVariables|GetGetIndex)))))))