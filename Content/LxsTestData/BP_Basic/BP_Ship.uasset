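; Racing dragon boat for a match-3 game, player or tag-identified AI, driven forward by ProjectileMovement with rower animation rate following speed.
; Tick eases speed toward base plus timestamp-stacked buffs and debuffs, or to zero at race end.
; Five skills apply boost, whirlpool spin, fog, chain or debuff immunity; fog and chain hit the player's HUD but suppress AI speed-ups.
; Difficulty sets AI delay range and bonus.
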(event Custom|Event_GetSpeedUP
  (params (BuffCount :type Integer) (SpeedUpAmount :type Float%20%28double-precision%29))
  ;[1 1 1] 执行加速效果
  (Components|Activation|SetActive (Variables|Default|GetSpeedUp1) true true)
  (Variables|Default|SetSpeed%20Up%20Amount SpeedUpAmount)
  (for _index (range 0 (- BuffCount 1))
    (Utilities|Array|Add (Variables|BuffTimer|GetSpeedUPBuffTimeSticks) (Utilities|Time|GetGameTimeinSeconds))))

(event Custom|Event_ChangeDifficulty
  (params (InputDifficulty :type EDifficultyLevel%20Enum :default "Easy"))
  ;[1 1 1] AI 难度更改
  (Utilities|FlowControl|Sequence
    (:then_0
      (|配置不同的延时效果_2 InputDifficulty))
    (:then_1
      (switch Utilities|FlowControl|Switch|SwitchonEDifficultyLevel InputDifficulty
        (:Easy
          ;;[1 1 1] 0/2/4/8/16
          (Variables|Default|SetDiffcultyAdd 0))
        (:Normal
          (Variables|Default|SetDiffcultyAdd 2))
        (:Hard
          (Variables|Default|SetDiffcultyAdd 4))
        (:Insane
          (Variables|Default|SetDiffcultyAdd 8))
        (:Hell
          (Variables|Default|SetDiffcultyAdd 16))))))

(event Custom|Event_RaceEnd
  ;[1 1 1] 结束游戏
  (Variables|Default|SetRaceEnd true))

(event Custom|Event_GetSpeedDown
  (params (BuffCount :type Integer) (SppedDownAmount :type Float%20%28double-precision%29))
  ;[1 1 1] 执行加速效果
  (if (not (Variables|Default|GetGolden%20body))
    (Variables|Default|SetSeedDownAmount SppedDownAmount)
    (for _index (range 0 (- BuffCount 1))
      (Utilities|Array|Add (Variables|BuffTimer|GetSpeedDownDebuffTimeSticks) (Utilities|Time|GetGameTimeinSeconds)))))

(event Custom|Event_ApplySkill
  (params (InputSkillType :type ESkillType%20Enum :default "EastWind") (SkillConfig :type Skill%20Config%20Structure) (TargetSelf :type Boolean))
  ;[1 1 1] 应用技能效果
  (switch Utilities|FlowControl|Switch|SwitchonESkillType InputSkillType
    (:EastWind
      (|借东风效果 SkillConfig))
    (:FloodSeven
      (|漩涡效果 SkillConfig))
    (:HeavyFog
      (|大雾效果 SkillConfig))
    (:IronChain
      (|铁锁连环效果 SkillConfig))
    (:EmptyCity
      (|金身效果 SkillConfig))))

(event Custom|Event_StartRace
  ;[1 1 1] 开始比赛
  (Variables|/Script/Engine.MovementComponent|SetVelocity (Variables|Default|GetProjectileMovement) (* (Math|Vector|GetForwardVector (Variables|Default|GetArrow)) (Variables|Default|GetNowSpeed)))
  (Components|Timeline|SetPlayRate (Variables|Default|GetSkeletalMesh1) 1.0)
  (Variables|Default|SetRaceStart true))

(event EventBeginPlay
  ;[1 1 1] 初始化
  (Components|Timeline|SetPlayRate (Variables|Default|GetSkeletalMesh1) 0.0)
  (bind _returnvalue (Actor|GetActorOfClass "/Game/BluePrint/Manager/BP_Match3Manager.BP_Match3Manager_C"))
  (Variables|Default|SetManager _returnvalue)
  (bind _aswbp_board_speed (Utilities|Casting|CastToWBP_BoardSpeed (UserInterface|GetWidget (Variables|Default|GetWidget))))
  (bind _output_get (Variables|Default|SetAs%20WBP%20Board%20Speed _aswbp_board_speed))
  (Variables|/Game/UMG/WBP_BoardSpeed.WBP_BoardSpeed_C|SetBindShip _output_get self)
  (Rendering|SetVisibility (Variables|Skill|GetDongFeng) false false))

(event Collision|EventActorBeginOverlap
  (params (OtherActor :type Actor%20Object%20Reference)))

(event EventTick
  (params (DeltaSeconds :type Float%20%28single-precision%29))
  ;[1 1 1] TicK
  (Variables|Default|SetDelta%20Seconds DeltaSeconds)
  (Utilities|FlowControl|Sequence
    (:then_0
      (if (Variables|SkillTimer|GetInFloodEffect)
        (Transformation|AddRelativeRotation (Variables|Default|GetStaticMesh) "0.000000,4.000000,0.000000" false false)
        (else
          (Transformation|SetRelativeRotation (Variables|Default|GetStaticMesh) (Math|Interpolation|RInterpTo (.rotation (Transformation|GetRelativeTransform (Variables|Default|GetStaticMesh))) "0.000000,-90.000000,0.000000" (Variables|Default|GetDelta%20Seconds) 3.0) false false)
          (if (Variables|Default|GetRaceStart)
            (Variables|Default|SetNowSpeed (select (Variables|Default|GetRaceEnd) (Math|Interpolation|FInterptoConstant (Variables|Default|GetNowSpeed) 0.0 (Variables|Default|GetDelta%20Seconds) (+ (/ (Variables|Default|GetNowSpeed) 5.0) 3e+02)) (Math|Interpolation|FInterptoConstant (Variables|Default|GetNowSpeed) (CallFunction|FGetFinalSpeed) (Variables|Default|GetDelta%20Seconds) (Utilities|Select :Index (Utilities|Array|Length (Variables|SkillTimer|GetDongFengTimer)) :Option%200 1e+02 :Option%201 3e+02))))
            ;;[1 1 1] 处理角色的播放速度
            (Components|Timeline|SetPlayRate (Variables|Default|GetSkeletalMesh1) (Math|Float|Clamp(Float) (/ (Variables|Default|GetNowSpeed) 2e+02) 0.0 1e+01))
            ;;[1 1 1] 处理速度中的内容
            (Variables|/Script/Engine.MovementComponent|SetVelocity (Variables|Default|GetProjectileMovement) (* (Math|Vector|GetForwardVector (Variables|Default|GetArrow)) (Variables|Default|GetNowSpeed)))))))))

(fn ConstructionScript)

(fn FGetBuffCount
  (params (InputTimeSticks :type Array%20of%20Floats%20%28double-precision%29) (BuffContiniutime :type Float%20%28double-precision%29))
  (bind _output_get (LocalVariables|SetCacheTimeStick InputTimeSticks))
  (for _array_element _output_get
    (if (<= (+ _array_element BuffContiniutime) (Utilities|Time|GetGameTimeinSeconds))
      (Utilities|Array|Add (LocalVariables|GetDeletTImerStick) _array_element)))
  (for _array_element_2 (LocalVariables|GetDeletTImerStick)
    (if (Utilities|Array|ContainsItem InputTimeSticks _array_element_2)
      (Utilities|Array|RemoveIndex InputTimeSticks (Utilities|Array|FindItem InputTimeSticks _array_element_2))))
  (return (Utilities|Array|Length InputTimeSticks)))

(fn FGetFinalSpeed
  (bind _manager (Variables|Default|GetManager))
  (bind _dongfengtimer (Variables|SkillTimer|GetDongFengTimer))
  (bind _skillconfigs (Variables|/Script/DragonBoat.Datamanagement|GetSkillConfigs _manager))
  (bind _value (Utilities|Map|Find _skillconfigs "EastWind"))
  (bind (_duration _effectvalue) (Utilities|Struct|BreakSkillConfig _value))
  (bind _outbuffcount (CallFunction|FGetBuffCount _dongfengtimer _duration))
  (if (>= _outbuffcount 1)
    _
    (else
      (Rendering|SetVisibility (Variables|Skill|GetDongFeng) false false)))
  (return (+ (+ (select (Variables|SkillTimer|GetInFogEffect) 0.0 (* (CallFunction|FGetBuffCount (Variables|BuffTimer|GetSpeedUPBuffTimeSticks) (Variables|/Game/BluePrint/Manager/BP_Match3Manager.BP_Match3Manager_C|GetSpeedUPtime (Variables|Default|GetManager))) (Variables|Default|GetSpeed%20Up%20Amount))) (* (CallFunction|FGetBuffCount (Variables|BuffTimer|GetSpeedDownDebuffTimeSticks) (Variables|/Game/BluePrint/Manager/BP_Match3Manager.BP_Match3Manager_C|GetSpeedDowntime (Variables|Default|GetManager))) (Variables|Default|GetSeedDownAmount) -1.0) (* _outbuffcount _effectvalue)) 0.0 (Variables|Default|GetBasicSpped))))

(fn FCheckSelfIsAI
  (return (or (Actor|ActorHasTag "AI01") (Actor|ActorHasTag "AI02"))))