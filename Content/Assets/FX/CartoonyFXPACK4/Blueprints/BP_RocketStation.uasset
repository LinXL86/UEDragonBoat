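; BP_RocketStation is a rocket station FX actor that plays a one-shot material animation on two stand components, then destroys itself.
; On BeginPlay, three chained timelines drive the "Anim" scalar parameter on dynamic material instances.
; Stand2 animates, swaps to a fuel material to animate again, then hides.
; Stand1 animates last, and the actor is destroyed after a short delay.
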(event EventBeginPlay
  (bind _stand2 (Variables|Default|GetStand2))
  (bind _stand1 (Variables|Default|GetStand1))
  (bind _stand2_2 (Variables|Default|GetStand2))
  (bind _returnvalue (Rendering|Material|CreateDynamicMaterialInstance _stand1 0 (Rendering|Material|GetMaterial _stand1 0) "None" :!class /Script/Engine.PrimitiveComponent))
  (bind _returnvalue_2 (Rendering|Material|CreateDynamicMaterialInstance _stand2_2 0 (Rendering|Material|GetMaterial _stand2_2 0) "None" :!class /Script/Engine.PrimitiveComponent))
  (bind _newtrack_0 (Timeline|Timeline_0 PlayFromStart)
    (:Update
      (Rendering|Material|SetScalarParameterValue _returnvalue_2 "Anim" _newtrack_0 :!class /Script/Engine.MaterialInstanceDynamic))
    (:Finished
      (Rendering|Material|SetMaterial _stand2 0 "/Game/Assets/FX/CartoonyFXPACK4/Materials/M_Stand2_Fuel_Inst1.M_Stand2_Fuel_Inst1")
      (bind _returnvalue_3 (Rendering|Material|CreateDynamicMaterialInstance _stand2 0 (Rendering|Material|GetMaterial _stand2 0) "None" :!class /Script/Engine.PrimitiveComponent))
      (bind _newtrack_0_2 (Timeline|Timeline_2 PlayFromStart)
        (:Update
          (Rendering|Material|SetScalarParameterValue _returnvalue_3 "Anim" _newtrack_0_2 :!class /Script/Engine.MaterialInstanceDynamic))
        (:Finished
          (Rendering|SetVisibility _stand2 false false)
          (bind _newtrack_0_3 (Timeline|Timeline_1 PlayFromStart)
            (:Update
              (Rendering|Material|SetScalarParameterValue _returnvalue "Anim" _newtrack_0_3 :!class /Script/Engine.MaterialInstanceDynamic))
            (:Finished
              (Utilities|FlowControl|Delay 1.0)
              (Actor|DestroyActor))))))))

(fn ConstructionScript)