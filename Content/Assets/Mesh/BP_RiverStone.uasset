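; BP_RiverStone is a spline-based placement Blueprint that generates a row of river stone meshes.
; Its construction script adds RiverStoneNum static mesh components, each randomly assigned one of the first three Stones meshes.
; Only relative X is set, by feeding an even fraction of spline length as a location into GetDistanceAlongSplineAtLocation, rather than sampling spline positions.
; The event graph has no active logic.
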(event EventBeginPlay)

(event Collision|EventActorBeginOverlap
  (params (OtherActor :type Actor%20Object%20Reference)))

(event EventTick
  (params (DeltaSeconds :type Float%20%28single-precision%29)))

(fn ConstructionScript
  (for _index (range 0 (- (Variables|Default|GetRiverStoneNum) 1))
    (bind _returnvalue (AddComponent|AddStaticMeshComponent false (Math|Transform|MakeTransform (Math|Vector|MakeVector (Class|SplineComponent|GetDistanceAlongSplineatLocation (Variables|Default|GetSpline) (Math|Vector|MakeVector (* (/ _index (Variables|Default|GetRiverStoneNum)) (Spline|GetSplineLength (Variables|Default|GetSpline))) 0.0 0.0) "Local") 0.0 0.0) "0, 0, 0" "1.000000,1.000000,1.000000")))
    (Components|StaticMesh|SetStaticMesh _returnvalue (Utilities|Array|Get(acopy) (Variables|Default|GetStones) (Math|Random|RandomIntegerinRange 0 2)))))